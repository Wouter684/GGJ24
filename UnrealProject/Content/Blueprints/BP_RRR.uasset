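; BP_RRR is an interactive music player that toggles its Music component on and off with IA_Use, restarting from the beginning each time.
; Overlapping its Trigger with BP_ThirdPersonCharacter shows ButtonPrompt and enables the actor's input for player 0.
; Leaving hides the prompt and calls DisableInput on the player controller itself, unlike the enable call, which targets this actor.
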(event OnComponentBeginOverlap(Trigger)
  (params (OverlappedComponent :type Primitive%20Component%20Object%20Reference) (OtherActor :type Actor%20Object%20Reference) (OtherComp :type Primitive%20Component%20Object%20Reference) (OtherBodyIndex :type Integer) (bFromSweep :type Boolean) (SweepResult :type Hit%20Result%20Structure%20%28by%20ref%29))
  (Utilities|Casting|CastToBP_ThirdPersonCharacter OtherActor)
  (Input|EnableInput (Game|GetPlayerController 0))
  (Rendering|SetVisibility (Variables|Default|GetButtonPrompt) true false))

(event OnComponentEndOverlap(Trigger)
  (params (OverlappedComponent :type Primitive%20Component%20Object%20Reference) (OtherActor :type Actor%20Object%20Reference) (OtherComp :type Primitive%20Component%20Object%20Reference) (OtherBodyIndex :type Integer))
  (Utilities|Casting|CastToBP_ThirdPersonCharacter OtherActor)
  (Input|DisableInput (Game|GetPlayerController 0) 0)
  (Rendering|SetVisibility (Variables|Default|GetButtonPrompt) false false))

(event Input|EnhancedActionEvents|EnhancedInputActionIA_Use
  (params (ActionValue :type Boolean) (ElapsedSeconds :type Float%20%28double-precision%29) (TriggeredSeconds :type Float%20%28double-precision%29) (InputAction :type Input%20Action%20Object%20Reference :default "/Game/ThirdPerson/Input/Actions/IA_Use.IA_Use"))
  (bind _music (Variables|Default|GetMusic))
  (:Started
    (if (Audio|Components|Audio|IsPlaying _music)
      (Audio|Components|Audio|Stop _music)
      (else
        (Audio|Components|Audio|Play _music 0.0)))))

(fn ConstructionScript)