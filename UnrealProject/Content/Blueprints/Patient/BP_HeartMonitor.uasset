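; Heart monitor prop that shows a patient's condition through beeps and an animated screen.
; UpdateHeartMonitor runs a timer whose beep interval interpolates with health ratio, so lower health beeps faster, and derives screen scroll speed from health.
; StopMonitor switches the screen mask for dead or cured patients and plays a flatline sound on death.
; A dynamic material instance created in the construction script drives the screen.
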(event Custom|Update%20Heart%20Monitor
  (params (Patient :type BP%20Hospital%20Bed%20Object%20Reference) (DeltaTime :type Float%20%28double-precision%29))
  ;[1 1 1] Update monitor
  (CallFunction|SetMonitorSpeed Patient)
  (CallFunction|SetMaxTime Patient)
  (if (>= (Variables|Default|GetcurrentTime) (Variables|Default|GetmaxTime))
    (Audio|Components|Audio|Play (Variables|Default|GetBeep) 0.0)
    (Variables|Default|SetcurrentTime 0.0)
    (else
      (Variables|Default|SetcurrentTime (+ (Variables|Default|GetcurrentTime) DeltaTime)))))

(event Custom|StopMonitor
  (params (Patient :type BP%20Hospital%20Bed%20Object%20Reference))
  (bind _beep (Variables|Default|GetBeep))
  ;[1 1 1] Patient dead/cured
  (if (Utilities|Enum|Equal(Enum) (Variables|/Game/Blueprints/Patient/BP_HospitalBed.BP_HospitalBed_C|GetStatus Patient) "NewEnumerator2")
    ;;[1 1 1] Dead
    (Audio|Components|Audio|SetSound _beep "/Game/SFX/Flatline.Flatline")
    (Audio|Components|Audio|Play _beep 0.0)
    (Variables|Default|SethasFlatlined true)
    (Rendering|Material|SetVectorParameterValue (Variables|Default|GetDynamicMaterial) "Mask" "(R=0.000000,G=1.000000,B=0.000000,A=1.000000)" :!class /Script/Engine.MaterialInstanceDynamic)
    (CallFunction|SetMonitorSpeed Patient)
    (else
      ;;[1 1 1] Cured
      (Variables|Default|SethasFlatlined true)
      (Rendering|Material|SetVectorParameterValue (Variables|Default|GetDynamicMaterial) "Mask" "(R=0.000000,G=0.000000,B=1.000000,A=1.000000)" :!class /Script/Engine.MaterialInstanceDynamic)
      (CallFunction|SetMonitorSpeed))))

(fn ConstructionScript
  (bind _returnvalue (Rendering|Material|CreateDynamicMaterialInstance (Rendering|Material|GetMaterial (Variables|Default|GetSM_Prop_Computer_Monitor_02) 1) "None" "None" :!class /Script/Engine.KismetMaterialLibrary))
  (bind _output_get (Variables|Default|SetDynamicMaterial _returnvalue))
  (Rendering|Material|SetMaterial (Variables|Default|GetSM_Prop_Computer_Monitor_02) 1 _output_get))

(fn SetMaxTime
  (params (Patient :type BP%20Hospital%20Bed%20Object%20Reference))
  (Variables|Default|SetmaxTime (+ (Variables|Default|GetlowestMaxTime) (* (/ (Variables|/Game/Blueprints/Patient/BP_HospitalBed.BP_HospitalBed_C|GetCurrentHealth Patient) (Variables|/Game/Blueprints/Patient/BP_HospitalBed.BP_HospitalBed_C|GetMaxHealth Patient)) (- (Variables|Default|GethighestMaxTime) (Variables|Default|GetlowestMaxTime))))))

(fn SetMonitorSpeed
  (params (Patient :type BP%20Hospital%20Bed%20Object%20Reference))
  (bind _dynamicmaterial (Variables|Default|GetDynamicMaterial))
  (if (Utilities|IsValid Patient)
    (if (== (Variables|/Game/Blueprints/Patient/BP_HospitalBed.BP_HospitalBed_C|GetCurrentHealth Patient) 0.0)
      (Rendering|Material|SetVectorParameterValue _dynamicmaterial "MonitorSpeed" (Utilities|Struct|MakeLinearColor 0.0 0.0 0.0 1.0) :!class /Script/Engine.MaterialInstanceDynamic)
      (else
        (Rendering|Material|SetVectorParameterValue _dynamicmaterial "MonitorSpeed" (Utilities|Struct|MakeLinearColor (- (LocalVariables|GetminSpeed) (* (- (LocalVariables|GetmaxSpeed) (LocalVariables|GetminSpeed)) (- 1.0 (/ (Variables|/Game/Blueprints/Patient/BP_HospitalBed.BP_HospitalBed_C|GetMaxHealth Patient) (Variables|/Game/Blueprints/Patient/BP_HospitalBed.BP_HospitalBed_C|GetCurrentHealth Patient))))) 0.0 0.0 1.0) :!class /Script/Engine.MaterialInstanceDynamic)))))