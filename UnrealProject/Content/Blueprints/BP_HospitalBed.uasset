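; Hospital bed with a randomly modelled patient, whom the player's clown heals with jokes before disease kills them.
; Tick drains health using disease data from GM_Main, drives the IV and heart monitor, and times infection, vomiting or manic episodes.
; ReceiveJoke heals more for favourite or disease super jokes, rejecting recent repeats and checking clown effects and Clownophobia outfit.
; ChangeHealth triggers cure at full health and death at zero.
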(event OnComponentEndOverlap(Box)
  (params (OverlappedComponent :type Primitive%20Component%20Object%20Reference) (OtherActor :type Actor%20Object%20Reference) (OtherComp :type Primitive%20Component%20Object%20Reference) (OtherBodyIndex :type Integer))
  (bind _clown (Variables|Default|GetClown))
  ;[1 1 1] Clown enter/exit box collision
  (if (== OtherActor _clown)
    (Variables|Default|SetClownIsClose false)
    (Variables|/Game/ThirdPerson/Blueprints/BP_ThirdPersonCharacter.BP_ThirdPersonCharacter_C|SetCurrentPatient _clown (Variables|Default|GetPatientNULL))
    (Variables|Default|SetDiseaseTimer 0.0)))

(event OnComponentBeginOverlap(Box)
  (params (OverlappedComponent :type Primitive%20Component%20Object%20Reference) (OtherActor :type Actor%20Object%20Reference) (OtherComp :type Primitive%20Component%20Object%20Reference) (OtherBodyIndex :type Integer) (bFromSweep :type Boolean) (SweepResult :type Hit%20Result%20Structure%20%28by%20ref%29))
  (bind _clown (Variables|Default|GetClown))
  ;[1 1 1] Clown enter/exit box collision
  (if (== OtherActor _clown)
    (Variables|Default|SetClownIsClose true)
    (Variables|/Game/ThirdPerson/Blueprints/BP_ThirdPersonCharacter.BP_ThirdPersonCharacter_C|SetCurrentPatient _clown self)))

(event Custom|PatientCured
  (bind _patient (Variables|Default|GetPatient))
  ;[1 1 1] Cure/Death
  (Default|StopMonitor (Variables|Default|GetMy%20Heart%20Monitor) self)
  (Transformation|SetRelativeLocation _patient "0.000000,100.000000,30.000000" false false)
  (Components|Animation|PlayAnimation _patient "/Game/Meshes/Animations/AS_NonPlayer/AS_SittingUp.AS_SittingUp" true)
  (CallFunction|RemoveDiseaseEffects false)
  (Utilities|FlowControl|Delay (Animation|GetPlayLength (Utilities|Struct|BreakSingleAnimationPlayData (Variables|/Script/Engine.SkeletalMeshComponent|GetAnimationData _patient))))
  (Components|Animation|PlayAnimation _patient "/Game/Meshes/Animations/AS_NonPlayer/AS_Idle_Sitting.AS_Idle_Sitting" true))

(event Custom|PatientDied
  (bind _patient (Variables|Default|GetPatient))
  ;[1 1 1] Cure/Death
  (Default|StopMonitor (Variables|Default|GetMy%20Heart%20Monitor) self)
  (Components|Animation|PlayAnimation _patient "/Game/Meshes/Animations/AS_NonPlayer/AS_Sleeping2.AS_Sleeping2" false)
  (Utilities|FlowControl|Delay 3.0)
  (Audio|Components|Audio|Stop _patient)
  (CallFunction|RemoveDiseaseEffects true))

(event Custom|Vomit
  (bind _patient (Variables|Default|GetPatient))
  (bind _animationdata (Variables|/Script/Engine.SkeletalMeshComponent|GetAnimationData _patient))
  (bind _animtoplay (Utilities|Struct|BreakSingleAnimationPlayData _animationdata))
  (bind _returnvalue (Animation|GetPlayLength _animtoplay))
  (bind _returnvalue_2 (/ _returnvalue 2.0))
  ;[1 1 1] Vomitting
  (Variables|Default|SetStatus "NewEnumerator3")
  (Components|Animation|PlayAnimation _patient "/Game/Meshes/Animations/AS_NonPlayer/AS_Vomitting.AS_Vomitting" false)
  (Components|Activation|Activate (Variables|Default|GetPart_Vomitting) false)
  (Utilities|FlowControl|Delay _returnvalue_2)
  (if (Variables|Default|GetClownIsClose)
    (Default|VomitOverClown (Variables|Default|GetClown)))
  (Utilities|FlowControl|Delay _returnvalue_2)
  (Components|Animation|PlayAnimation _patient "/Game/Meshes/Animations/AS_NonPlayer/AS_Nodding.AS_Nodding" true)
  (Variables|Default|SetDiseaseTimer 0.0)
  (Variables|Default|SetStatus "NewEnumerator0"))

(event Custom|ManicEpisode
  (bind _patient (Variables|Default|GetPatient))
  ;[1 1 1] Manic Episode
  (Variables|Default|SetStatus "NewEnumerator4")
  (Components|Animation|PlayAnimation _patient "/Game/Meshes/Animations/AS_Player/AS_Ymca_Dance.AS_Ymca_Dance" true)
  (Utilities|FlowControl|Delay (* (Animation|GetPlayLength (Utilities|Struct|BreakSingleAnimationPlayData (Variables|/Script/Engine.SkeletalMeshComponent|GetAnimationData _patient))) 3.0))
  (Components|Animation|PlayAnimation _patient "/Game/Meshes/Animations/AS_NonPlayer/AS_Shrugging.AS_Shrugging" true)
  (Variables|Default|SetDiseaseTimer 0.0)
  (Variables|Default|SetStatus "NewEnumerator0"))

(event EventBeginPlay
  (bind _jokesheardtimer (Variables|Default|GetJokesHeardTimer))
  ;[1 1 1] Begin Play
  (Utilities|FlowControl|Sequence
    (:then_0
      ;;[1 1 1] Set Clown
      (bind _asbp_third_person_character (Utilities|Casting|CastToBP_ThirdPersonCharacter (Game|GetPlayerCharacter 0)))
      (Variables|Default|SetClown _asbp_third_person_character))
    (:then_1
      ;;[1 1 1] Set Disease
      (CallFunction|SetDisease(Start)))
    (:then_2
      ;;[1 1 1] Set Jokes
      (for (_ _array_index) _jokesheardtimer
        (Utilities|Array|SetArrayElem _jokesheardtimer _array_index (Variables|Default|GetJokesHeardCooldown)))
      (bind _asw_patient_feedback (Utilities|Casting|CastToW_PatientFeedback (UserInterface|GetWidget (Variables|Default|GetW_PatientFeedback))))
      (bind _output_get (Variables|Default|SetW%20Patient%20Feedback _asw_patient_feedback))
      (Default|SetupFeedback _output_get self)
      (if (Utilities|Enum|Equal(Enum) (Variables|Default|GetFavouriteJoke) "NewEnumerator8")
        (Development|PrintString "a Patient has no fave joke" true true "(R=1.000000,G=0.000000,B=0.048679,A=1.000000)" 1e+01)))
    (:then_3
      ;;[1 1 1] Set current and max health
      (if (== (Variables|Default|GetMaxHealth) 0)
        (bind _output_get_2 (Variables|Default|SetMaxHealth 40)))
      (if (> (Variables|Default|GetCurrentHealth) (Math|Conversions|ToFloat(Integer) _output_get_2))
        (Variables|Default|SetCurrentHealth (Math|Conversions|ToFloat(Integer) _output_get_2))))
    (:then_4
      ;;[1 1 1] Find IV and Heart Monitor
      (bind _asbp_iv (Utilities|Casting|CastToBP_IV (Variables|/Script/Engine.ChildActorComponent|GetChildActor (Variables|Default|GetBP_IV)))
        (:then
          (Variables|Default|SetMyIV _asbp_iv))
        (:CastFailed
          _))
      (bind _asbp_heart_monitor (Utilities|Casting|CastToBP_HeartMonitor (Variables|/Script/Engine.ChildActorComponent|GetChildActor (Variables|Default|GetBP_HeartMonitor))))
      (Variables|Default|SetMy%20Heart%20Monitor _asbp_heart_monitor))))

(event EventTick
  (params (DeltaSeconds :type Float%20%28single-precision%29))
  (bind _self self)
  ;[1 1 1] Event Tick
  (Utilities|FlowControl|Sequence
    (:then_0
      ;;[1 1 1] Change patient Health
      (switch Utilities|FlowControl|Switch|SwitchonE_PatientStatus (Variables|Default|GetStatus)
        (:NewEnumerator0
          (Default|ChangeIVFill (Variables|Default|GetMyIV) _self)
          (Default|UpdateHeartMonitor (Variables|Default|GetMy%20Heart%20Monitor) _self DeltaSeconds)
          (CallFunction|DiseaseEffect DeltaSeconds)
          (CallFunction|ChangeHealth (* (* (Utilities|Struct|BreakBPS_Disease (Variables|Default|GetActive%20Disease)) DeltaSeconds) -1.0))
          (if (and (Variables|Default|GetClownIsClose) (> (Utilities|Array|Length (Variables|/Game/ThirdPerson/Blueprints/BP_ThirdPersonCharacter.BP_ThirdPersonCharacter_C|GetActiveEffects (Variables|Default|GetClown))) 0))
            (CallFunction|ChangeHealth 0.0)))))
    (:then_1
      ;;[1 1 1] Jokes heard timer
      (for (_array_element _array_index) (Variables|Default|GetJokesHeard)
        (if (Utilities|Enum|NotEqual(Enum) _array_element "NewEnumerator8")
          (if (<= (- (Utilities|Array|Get(acopy) (Variables|Default|GetJokesHeardTimer) _array_index) DeltaSeconds) 0.0)
            (Utilities|Array|SetArrayElem (Variables|Default|GetJokesHeard) _array_index "NewEnumerator8")
            (Utilities|Array|SetArrayElem (Variables|Default|GetJokesHeardTimer) _array_index (Variables|Default|GetJokesHeardCooldown))
            (else
              (Utilities|Array|SetArrayElem (Variables|Default|GetJokesHeardTimer) _array_index (- (Utilities|Array|Get(acopy) (Variables|Default|GetJokesHeardTimer) _array_index) DeltaSeconds)))))))))

(fn ConstructionScript
  (bind _returnvalue (Math|Random|RandomInteger 9))
  (Components|SkeletalMesh|SetSkeletalMeshAsset (Variables|Default|GetPatient) (Variables|Character|GetPatientModel))
  (Utilities|FlowControl|Sequence
    (:then_0
      ;[1 1 1] Set animation
      (switch Utilities|FlowControl|Switch|SwitchonE_Disease (Variables|Default|GetStart%20Disease)
        (:NewEnumerator0
          (Variables|/Script/Engine.SkeletalMeshComponent|SetAnimationData (Variables|Default|GetPatient) (Utilities|Struct|MakeSingleAnimationPlayData "/Game/Meshes/Animations/AS_NonPlayer/AS_Nodding.AS_Nodding" true true 0.0 1.0))
          (Rendering|SetVisibility (Variables|Default|GetCast) true false))
        (:NewEnumerator1
          (Variables|/Script/Engine.SkeletalMeshComponent|SetAnimationData (Variables|Default|GetPatient) (Utilities|Struct|MakeSingleAnimationPlayData "/Game/Meshes/Animations/AS_NonPlayer/AS_Moaning.AS_Moaning" true true 0.0 1.0)))
        (:NewEnumerator2
          (Variables|/Script/Engine.SkeletalMeshComponent|SetAnimationData (Variables|Default|GetPatient) (Utilities|Struct|MakeSingleAnimationPlayData "/Game/Meshes/Animations/AS_NonPlayer/AS_Nodding.AS_Nodding" true true 0.0 1.0)))
        (:NewEnumerator3
          (Variables|/Script/Engine.SkeletalMeshComponent|SetAnimationData (Variables|Default|GetPatient) (Utilities|Struct|MakeSingleAnimationPlayData "/Game/Meshes/Animations/AS_NonPlayer/AS_Coughing_Severe.AS_Coughing_Severe" true true 0.0 1.0)))
        (:NewEnumerator4
          (Variables|/Script/Engine.SkeletalMeshComponent|SetAnimationData (Variables|Default|GetPatient) (Utilities|Struct|MakeSingleAnimationPlayData "/Game/Meshes/Animations/AS_NonPlayer/AS_Shrugging.AS_Shrugging" true true 0.0 1.0) :!label _label))
        (:NewEnumerator5
          (goto _label))))
    (:then_1
      ;[1 1 1] Set Mesh
      (switch int _returnvalue
        (:Default
          (Development|PrintString (Utilities|String|Append "Exceded max value! " (Utilities|String|ToString(Integer) _returnvalue)) true true "(R=1.000000,G=0.000000,B=0.000000,A=1.000000)" 5.0))
        (:0
          (Components|SkeletalMesh|SetSkeletalMeshAsset (Variables|Default|GetPatient) "/Game/PolygonTown/Meshes/Characters/SK_Character_Daughter_01.SK_Character_Daughter_01"))
        (:1
          (Components|SkeletalMesh|SetSkeletalMeshAsset (Variables|Default|GetPatient) "/Game/PolygonTown/Meshes/Characters/SK_Character_Father_01.SK_Character_Father_01"))
        (:2
          (Components|SkeletalMesh|SetSkeletalMeshAsset (Variables|Default|GetPatient) "/Game/PolygonTown/Meshes/Characters/SK_Character_Daughter_01.SK_Character_Daughter_01"))
        (:3
          (Components|SkeletalMesh|SetSkeletalMeshAsset (Variables|Default|GetPatient) "/Game/PolygonTown/Meshes/Characters/SK_Character_Mother_01.SK_Character_Mother_01"))
        (:4
          (Components|SkeletalMesh|SetSkeletalMeshAsset (Variables|Default|GetPatient) "/Game/PolygonTown/Meshes/Characters/SK_Character_Mother_02.SK_Character_Mother_02"))
        (:5
          (Components|SkeletalMesh|SetSkeletalMeshAsset (Variables|Default|GetPatient) "/Game/PolygonTown/Meshes/Characters/SK_Character_SchoolBoy_01.SK_Character_SchoolBoy_01"))
        (:6
          (Components|SkeletalMesh|SetSkeletalMeshAsset (Variables|Default|GetPatient) "/Game/PolygonTown/Meshes/Characters/SK_Character_SchoolGirl_01.SK_Character_SchoolGirl_01"))
        (:7
          (Components|SkeletalMesh|SetSkeletalMeshAsset (Variables|Default|GetPatient) "/Game/PolygonTown/Meshes/Characters/SK_Character_ShopKeeper_01.SK_Character_ShopKeeper_01"))
        (:8
          (Components|SkeletalMesh|SetSkeletalMeshAsset (Variables|Default|GetPatient) "/Game/PolygonTown/Meshes/Characters/SK_Character_Son_01.SK_Character_Son_01"))))))

(fn ReceiveJoke
  (params (HealBy :type Float%20%28double-precision%29) (UsedJoke :type E_Joke%20Enum :default "NewEnumerator8") (Character%20Joke :type Widget%20Component%20Object%20Reference))
  (LocalVariables|SetHealByVar HealBy)
  (LocalVariables|SetUsedJokeVar UsedJoke)
  (LocalVariables|SetCharacterJokePopup Character%20Joke)
  (if (and (== (Utilities|Array|Length (Variables|/Game/ThirdPerson/Blueprints/BP_ThirdPersonCharacter.BP_ThirdPersonCharacter_C|GetActiveEffects (Variables|Default|GetClown))) 0) (or (Class|KismetMathLibrary|XORBoolean (Utilities|Enum|Equal(Enum) "NewEnumerator0" (Utilities|Struct|BreakBPS_Outfit (Variables|/Game/ThirdPerson/Blueprints/BP_ThirdPersonCharacter.BP_ThirdPersonCharacter_C|GetCurrentOutfit (Variables|Default|GetClown)))) (Utilities|Enum|Equal(Enum) "NewEnumerator4" (Utilities|Struct|BreakBPS_Disease (Variables|Default|GetActive%20Disease)))) (Utilities|Enum|NotEqual(Enum) (Utilities|Struct|BreakBPS_Disease (Variables|Default|GetActive%20Disease)) "NewEnumerator4")))
    ;[1 1 1] Check for double jokes
    (bind _array_element (Utilities|Array|ForEachLoopwithBreak (Variables|Default|GetJokesHeard) :!label _label)
      (:LoopBody
        (if (Utilities|Enum|Equal(Enum) _array_element (LocalVariables|GetUsedJokeVar))
          (LocalVariables|SetisDouble true)
          (goto _label Break)))
      (:Completed
        (if (LocalVariables|GetisDouble)
          ;[1 1 1] Show sad feedback
          (Default|ShowJokeFeedback (Variables|Default|GetW%20Patient%20Feedback) false)
          (else
            ;[1 1 1] Change health
            (if (and (Utilities|Enum|Equal(Enum) (Variables|Default|GetFavouriteJoke) (LocalVariables|GetUsedJokeVar)) (Utilities|Enum|Equal(Enum) (LocalVariables|GetUsedJokeVar) (Utilities|Struct|BreakBPS_Disease (Variables|Default|GetActive%20Disease))))
              (CallFunction|ChangeHealth (* (LocalVariables|GetHealByVar) 3.0))
              (elif (Class|KismetMathLibrary|XORBoolean (Utilities|Enum|Equal(Enum) (Variables|Default|GetFavouriteJoke) (LocalVariables|GetUsedJokeVar)) (Utilities|Enum|Equal(Enum) (LocalVariables|GetUsedJokeVar) (Utilities|Struct|BreakBPS_Disease (Variables|Default|GetActive%20Disease))))
                (CallFunction|ChangeHealth (* (LocalVariables|GetHealByVar) 2.0))
                (else
                  (CallFunction|ChangeHealth (LocalVariables|GetHealByVar)))))
            ;[1 1 1] Add to jokes heard
            (bind (_array_element_2 _array_index) (Utilities|Array|ForEachLoopwithBreak (Variables|Default|GetJokesHeard) :!label _label_2)
              (:LoopBody
                (if (Utilities|Enum|Equal(Enum) _array_element_2 "NewEnumerator8")
                  (Utilities|Array|SetArrayElem (Variables|Default|GetJokesHeard) _array_index (LocalVariables|GetUsedJokeVar))
                  (goto _label_2 Break)))
              (:Completed
                ;[1 1 1] Show happy feedback
                (Default|ShowJokeFeedback (Variables|Default|GetW%20Patient%20Feedback) true)))))))
    (else
      (Default|ShowJokeFeedback (Variables|Default|GetW%20Patient%20Feedback) false))))

(fn ChangeHealth
  (params (Change :type Float%20%28double-precision%29))
  (bind _maxhealth (Variables|Default|GetMaxHealth))
  (bind _returnvalue (Math|Conversions|ToFloat(Integer) _maxhealth))
  (bind _output_get (Variables|Default|SetCurrentHealth (Math|Float|Clamp(Float) (+ Change (Variables|Default|GetCurrentHealth)) 0.0 _returnvalue)))
  (if (== _output_get 0.0)
    (Variables|Default|SetStatus "NewEnumerator2")
    (CallFunction|PatientDied)
    (elif (== _output_get _returnvalue)
      (Variables|Default|SetStatus "NewEnumerator1")
      (CallFunction|PatientCured))))

(fn DiseaseEffect
  (params (DeltaTime :type Float%20%28double-precision%29))
  (bind _clown (Variables|Default|GetClown))
  (LocalVariables|SetDelta%20Time DeltaTime)
  (if (and (Utilities|Enum|NotEqual(Enum) (Utilities|Struct|BreakBPS_Disease (Variables|Default|GetActive%20Disease)) "NewEnumerator3") (>= (Variables|Default|GetCurrentHealth) (* (Utilities|Struct|BreakBPS_Disease (Variables|Default|GetActive%20Disease)) 5.0)))
    (switch Utilities|FlowControl|Switch|SwitchonE_ClownEffects (Utilities|Struct|BreakBPS_Disease (Variables|Default|GetActive%20Disease))
      (:NewEnumerator1
        ;[1 1 1] Plague effect
        (if (Math|Boolean|ANDBoolean (not (Utilities|Array|ContainsItem (Variables|/Game/ThirdPerson/Blueprints/BP_ThirdPersonCharacter.BP_ThirdPersonCharacter_C|GetActiveEffects _clown) "NewEnumerator1")) (Variables|Default|GetClownIsClose) (Utilities|Enum|NotEqual(Enum) (Utilities|Struct|BreakBPS_Outfit (Variables|/Game/ThirdPerson/Blueprints/BP_ThirdPersonCharacter.BP_ThirdPersonCharacter_C|GetCurrentOutfit _clown)) "NewEnumerator2"))
          (bind _output_get (Variables|Default|SetDiseaseTimer (+ (LocalVariables|GetDelta%20Time) (Variables|Default|GetDiseaseTimer))))
          (if (>= _output_get (Utilities|Struct|BreakBPS_Disease (Variables|Default|GetActive%20Disease)))
            (Default|InfectClown (Variables|Default|GetClown))
            (Variables|Default|SetDiseaseTimer 0.0))))
      (:NewEnumerator2
        ;[1 1 1] Vomitting
        (if (and (not (Utilities|Array|ContainsItem (Variables|/Game/ThirdPerson/Blueprints/BP_ThirdPersonCharacter.BP_ThirdPersonCharacter_C|GetActiveEffects (Variables|Default|GetClown)) "NewEnumerator2")) (Utilities|Enum|NotEqual(Enum) (Variables|Default|GetStatus) "NewEnumerator3"))
          (bind _output_get_2 (Variables|Default|SetDiseaseTimer (+ (LocalVariables|GetDelta%20Time) (Variables|Default|GetDiseaseTimer))))
          (if (>= _output_get_2 (Utilities|Struct|BreakBPS_Disease (Variables|Default|GetActive%20Disease)))
            (CallFunction|Vomit))))
      (:NewEnumerator4
        ;[1 1 1] Manic Episode
        (if (Utilities|Enum|NotEqual(Enum) (Variables|Default|GetStatus) "NewEnumerator4")
          (bind _output_get_3 (Variables|Default|SetDiseaseTimer (+ (LocalVariables|GetDelta%20Time) (Variables|Default|GetDiseaseTimer))))
          (if (>= _output_get_3 (Utilities|Struct|BreakBPS_Disease (Variables|Default|GetActive%20Disease)))
            (CallFunction|ManicEpisode)))))))

(fn SetDisease(Start)
  (bind _asgm_main (Utilities|Casting|CastToGM_Main (Game|GetGameMode)))
  (bind _disease_struct (Default|GetDisease _asgm_main (Variables|Default|GetStart%20Disease)))
  (bind _output_get (Variables|Default|SetActive%20Disease _disease_struct))
  (switch Utilities|FlowControl|Switch|SwitchonE_Disease (Utilities|Struct|BreakBPS_Disease _output_get)
    (:NewEnumerator3
      (Components|Activation|Activate (Variables|Default|GetPart_Infected) false))))

(fn RemoveDiseaseEffects
  (params (Is%20Dead :type Boolean))
  (LocalVariables|SetHas%20Died Is%20Dead)
  (switch Utilities|FlowControl|Switch|SwitchonE_Disease (Utilities|Struct|BreakBPS_Disease (Variables|Default|GetActive%20Disease))
    (:NewEnumerator0
      (if (not (LocalVariables|GetHas%20Died))
        (Rendering|SetVisibility (Variables|Default|GetCast) false false)))
    (:NewEnumerator3
      (Components|Activation|Deactivate (Variables|Default|GetPart_Infected)))))