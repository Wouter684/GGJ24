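; BP_Suitcase is an interactable suitcase where the clown player picks jokes to assign to three joke slots.
; Its trigger box enables input and shows a button prompt while the player overlaps.
; Input actions toggle the HUD's joke inventory, navigate selection and pages, and assign the selected joke to the clown.
; SetAvailableJokes deduplicates its joke list, filters the GameMode's jokes against it, and fills the inventory widget.
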(event OnComponentBeginOverlap(TriggerBox)
  (params (OverlappedComponent :type Primitive%20Component%20Object%20Reference) (OtherActor :type Actor%20Object%20Reference) (OtherComp :type Primitive%20Component%20Object%20Reference) (OtherBodyIndex :type Integer) (bFromSweep :type Boolean) (SweepResult :type Hit%20Result%20Structure%20%28by%20ref%29))
  ;[1 1 1] Player enters hitbox
  (bind _asbp_third_person_character (Utilities|Casting|CastToBP_ThirdPersonCharacter OtherActor))
  (Variables|Default|SetClown _asbp_third_person_character)
  (Input|EnableInput (Game|GetPlayerController 0))
  (Rendering|SetVisibility (Variables|Default|GetButtonPrompt) true false))

(event OnComponentEndOverlap(TriggerBox)
  (params (OverlappedComponent :type Primitive%20Component%20Object%20Reference) (OtherActor :type Actor%20Object%20Reference) (OtherComp :type Primitive%20Component%20Object%20Reference) (OtherBodyIndex :type Integer))
  ;[1 1 1] Player enters hitbox
  (Utilities|Casting|CastToBP_ThirdPersonCharacter OtherActor)
  (Input|DisableInput (Game|GetPlayerController 0))
  (Rendering|SetVisibility (Variables|Default|GetButtonPrompt) false false))

(event Input|EnhancedActionEvents|EnhancedInputActionIA_Use
  (params (ActionValue :type Boolean) (ElapsedSeconds :type Float%20%28double-precision%29) (TriggeredSeconds :type Float%20%28double-precision%29) (InputAction :type Input%20Action%20Object%20Reference :default "/Game/ThirdPerson/Input/Actions/IA_Use.IA_Use"))
  ;[1 1 1] Show / Hide inventory
  (:Started
    (Default|OpenCloseJokeInventory (Variables|Default|GetW%20Main%20HUD) self (Variables|Default|GetClown))
    (bind _selected_joke (CallFunction|GetSelectedJoke))
    (Variables|Default|SetSelectedJoke _selected_joke)))

(event Input|EnhancedActionEvents|EnhancedInputActionIA_Item1
  (params (ActionValue :type Boolean) (ElapsedSeconds :type Float%20%28double-precision%29) (TriggeredSeconds :type Float%20%28double-precision%29) (InputAction :type Input%20Action%20Object%20Reference :default "/Game/ThirdPerson/Input/Actions/IA_Item1.IA_Item1"))
  ;[1 1 1] Set Jokes
  ;;[1 1 1] Set Joke 1
  (:Started
    (if (Variables|Default|GetIs%20Open)
      (Default|SetJokeFunc (Variables|Default|GetClown) 0 (Variables|Default|GetSelectedJoke)))))

(event Input|EnhancedActionEvents|EnhancedInputActionIA_Item2
  (params (ActionValue :type Boolean) (ElapsedSeconds :type Float%20%28double-precision%29) (TriggeredSeconds :type Float%20%28double-precision%29) (InputAction :type Input%20Action%20Object%20Reference :default "/Game/ThirdPerson/Input/Actions/IA_Item2.IA_Item2"))
  ;[1 1 1] Set Jokes
  ;;[1 1 1] Set Joke 2
  (:Started
    (if (Variables|Default|GetIs%20Open)
      (Default|SetJokeFunc (Variables|Default|GetClown) 1 (Variables|Default|GetSelectedJoke)))))

(event Input|EnhancedActionEvents|EnhancedInputActionIA_JokePageNext
  (params (ActionValue :type Boolean) (ElapsedSeconds :type Float%20%28double-precision%29) (TriggeredSeconds :type Float%20%28double-precision%29) (InputAction :type Input%20Action%20Object%20Reference :default "/Game/ThirdPerson/Input/Actions/IA_JokePageNext.IA_JokePageNext"))
  ;[1 1 1] Change page
  (:Started
    (if (Variables|Default|GetIs%20Open)
      (Default|ChangePage (Variables|Default|GetW%20Joke%20Inventory) 1)
      (bind _selected_joke (CallFunction|GetSelectedJoke))
      (Variables|Default|SetSelectedJoke _selected_joke))))

(event Input|EnhancedActionEvents|EnhancedInputActionIA_UI_Down
  (params (ActionValue :type Boolean) (ElapsedSeconds :type Float%20%28double-precision%29) (TriggeredSeconds :type Float%20%28double-precision%29) (InputAction :type Input%20Action%20Object%20Reference :default "/Game/ThirdPerson/Input/Actions/IA_UI_Down.IA_UI_Down"))
  ;[1 1 1] Navigation
  (:Started
    (Default|ChangeSelection (Variables|Default|GetW%20Joke%20Inventory) 0 1)
    (bind _selected_joke (CallFunction|GetSelectedJoke))
    (Variables|Default|SetSelectedJoke _selected_joke)))

(event Input|EnhancedActionEvents|EnhancedInputActionIA_UI_Up
  (params (ActionValue :type Boolean) (ElapsedSeconds :type Float%20%28double-precision%29) (TriggeredSeconds :type Float%20%28double-precision%29) (InputAction :type Input%20Action%20Object%20Reference :default "/Game/ThirdPerson/Input/Actions/IA_UI_Up.IA_UI_Up"))
  ;[1 1 1] Navigation
  (:Started
    (Default|ChangeSelection (Variables|Default|GetW%20Joke%20Inventory) 0 -1)
    (bind _selected_joke (CallFunction|GetSelectedJoke))
    (Variables|Default|SetSelectedJoke _selected_joke)))

(event Input|EnhancedActionEvents|EnhancedInputActionIA_Item3
  (params (ActionValue :type Boolean) (ElapsedSeconds :type Float%20%28double-precision%29) (TriggeredSeconds :type Float%20%28double-precision%29) (InputAction :type Input%20Action%20Object%20Reference :default "/Game/ThirdPerson/Input/Actions/IA_Item3.IA_Item3"))
  ;[1 1 1] Set Jokes
  ;;[1 1 1] Set Joke 3
  (:Started
    (if (Variables|Default|GetIs%20Open)
      (Default|SetJokeFunc (Variables|Default|GetClown) 2 (Variables|Default|GetSelectedJoke)))))

(event Input|EnhancedActionEvents|EnhancedInputActionIA_UI_Left
  (params (ActionValue :type Boolean) (ElapsedSeconds :type Float%20%28double-precision%29) (TriggeredSeconds :type Float%20%28double-precision%29) (InputAction :type Input%20Action%20Object%20Reference :default "/Game/ThirdPerson/Input/Actions/IA_UI_Left.IA_UI_Left"))
  ;[1 1 1] Navigation
  (:Started
    (Default|ChangeSelection (Variables|Default|GetW%20Joke%20Inventory) -1)
    (bind _selected_joke (CallFunction|GetSelectedJoke))
    (Variables|Default|SetSelectedJoke _selected_joke)))

(event Input|EnhancedActionEvents|EnhancedInputActionIA_JokePagePrevious
  (params (ActionValue :type Boolean) (ElapsedSeconds :type Float%20%28double-precision%29) (TriggeredSeconds :type Float%20%28double-precision%29) (InputAction :type Input%20Action%20Object%20Reference :default "/Game/ThirdPerson/Input/Actions/IA_JokePagePrevious.IA_JokePagePrevious"))
  ;[1 1 1] Change page
  (:Started
    (if (Variables|Default|GetIs%20Open)
      (Default|ChangePage (Variables|Default|GetW%20Joke%20Inventory) -1)
      (bind _selected_joke (CallFunction|GetSelectedJoke))
      (Variables|Default|SetSelectedJoke _selected_joke))))

(event Input|EnhancedActionEvents|EnhancedInputActionIA_UI_Right
  (params (ActionValue :type Boolean) (ElapsedSeconds :type Float%20%28double-precision%29) (TriggeredSeconds :type Float%20%28double-precision%29) (InputAction :type Input%20Action%20Object%20Reference :default "/Game/ThirdPerson/Input/Actions/IA_UI_Right.IA_UI_Right"))
  ;[1 1 1] Navigation
  (:Started
    (Default|ChangeSelection (Variables|Default|GetW%20Joke%20Inventory) 1)
    (bind _selected_joke (CallFunction|GetSelectedJoke))
    (Variables|Default|SetSelectedJoke _selected_joke)))

(fn ConstructionScript)

(fn SetAvailableJokes
  (params (Game%20Mode :type GM%20Main%20Object%20Reference))
  (Utilities|FlowControl|Sequence
    (:then_0
      (bind _output_get (Variables|Default|SetW%20Main%20HUD (Variables|/Game/Blueprints/Core/GM_Main.GM_Main_C|GetW_MainHUD_REF Game%20Mode)))
      (Variables|Default|SetW%20Joke%20Inventory (Variables|/Game/HUD/W_MainHUD.W_MainHUD_C|GetW_JokeInventory _output_get)))
    (:then_1
      (CallFunction|RemoveDoubleJokes)
      (for _array_element (Variables|/Game/Blueprints/Core/GM_Main.GM_Main_C|GetAllJokes Game%20Mode)
        (bind _output_get_2 (LocalVariables|SetLoop%20Joke _array_element))
        (if (Utilities|Array|ContainsItem (Variables|Default|GetAvailable%20Jokes) (.Name (Utilities|Struct|BreakBPS_Joke _output_get_2)))
          (Utilities|Array|Add (Variables|Default|GetJokes%20in%20suitcase) (LocalVariables|GetLoop%20Joke))))
      (Default|SetupJokeInventory (Variables|Default|GetW%20Joke%20Inventory) (Variables|Default|GetJokes%20in%20suitcase)))))

(fn RemoveDoubleJokes
  (for _array_element (Variables|Default|GetAvailable%20Jokes)
    (if (Utilities|Enum|NotEqual(Enum) _array_element "NewEnumerator8")
      (Utilities|Array|AddUnique (LocalVariables|GetNew%20Available%20Jokes) _array_element)))
  (Variables|Default|SetAvailable%20Jokes (LocalVariables|GetNew%20Available%20Jokes)))

(fn GetSelectedJoke
  (bind _array_element (Utilities|Array|ForEachLoopwithBreak (Variables|Default|GetJokes%20in%20suitcase) :!label _label)
    (:LoopBody
      (if (Utilities|Enum|Equal(Enum) (Variables|/Game/HUD/W_JokeInventory.W_JokeInventory_C|GetSelectedJoke (Variables|Default|GetW%20Joke%20Inventory)) (.Name (Utilities|Struct|BreakBPS_Joke _array_element)))
        (LocalVariables|SetJoke _array_element)
        (goto _label Break)))
    (:Completed
      (if (Utilities|Enum|NotEqual(Enum) (.Name (Utilities|Struct|BreakBPS_Joke (LocalVariables|GetJoke))) "NewEnumerator8")
        (return (LocalVariables|GetJoke))
        (else
          (Development|PrintString "Invalid joke selected!" true true "(R=1.000000,G=0.000000,B=0.000000,A=1.000000)"))))))