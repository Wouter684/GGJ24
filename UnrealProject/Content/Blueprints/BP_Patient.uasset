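; Patient actor that starts sick and changes health over time according to its disease, becoming dead at zero health or cured at full.
; An overlap box registers it as the clown player's current patient while the clown is near.
; Received jokes heal it, doubly if the joke is its favourite.
; Plague also infects a nearby clown once accumulated exposure time reaches a threshold.
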(event OnComponentEndOverlap(Box)
  (params (OverlappedComponent :type Primitive%20Component%20Object%20Reference) (OtherActor :type Actor%20Object%20Reference) (OtherComp :type Primitive%20Component%20Object%20Reference) (OtherBodyIndex :type Integer))
  (bind _clown (Variables|Default|GetClown))
  (if (== OtherActor _clown)
    (Development|PrintString "Bye bye")
    (Variables|Default|SetClownIsClose false)
    (Variables|/Game/ThirdPerson/Blueprints/BP_ThirdPersonCharacter.BP_ThirdPersonCharacter_C|SetCurrentPatient _clown (Variables|Default|GetPatientNULL))))

(event OnComponentBeginOverlap(Box)
  (params (OverlappedComponent :type Primitive%20Component%20Object%20Reference) (OtherActor :type Actor%20Object%20Reference) (OtherComp :type Primitive%20Component%20Object%20Reference) (OtherBodyIndex :type Integer) (bFromSweep :type Boolean) (SweepResult :type Hit%20Result%20Structure%20%28by%20ref%29))
  (bind _clown (Variables|Default|GetClown))
  (if (== OtherActor _clown)
    (Development|PrintString "Hello")
    (Variables|Default|SetClownIsClose true)
    (Variables|/Game/ThirdPerson/Blueprints/BP_ThirdPersonCharacter.BP_ThirdPersonCharacter_C|SetCurrentPatient _clown self)))

(event EventBeginPlay
  (bind _asbp_third_person_character (Utilities|Casting|CastToBP_ThirdPersonCharacter (Game|GetPlayerCharacter 0)))
  (Variables|Default|SetClown _asbp_third_person_character)
  (if (Utilities|Enum|Equal(Enum) (Variables|Default|GetStatus) "NewEnumerator0")
    _
    (else
      (Variables|Default|SetStatus "NewEnumerator0")))
  (if (Utilities|Enum|Equal(Enum) (Variables|Default|GetFavouriteJoke) "NewEnumerator8")
    (Development|PrintString "a Patient has no fave joke" true true "(R=1.000000,G=0.000000,B=0.048679,A=1.000000)" 1e+01)))

(event Collision|EventActorBeginOverlap
  (params (OtherActor :type Actor%20Object%20Reference)))

(event EventTick
  (params (DeltaSeconds :type Float%20%28single-precision%29))
  (switch Utilities|FlowControl|Switch|SwitchonE_PatientStatus "NewEnumerator0"
    (:NewEnumerator0
      (switch Utilities|FlowControl|Switch|SwitchonE_Diseases (Variables|Default|GetHasDisease)
        (:NewEnumerator0
          (bind _result (Math|Float|NegateFloat (* DeltaSeconds 0.5))
            (:%20%20
              (CallFunction|ChangeHealth _result))))
        (:NewEnumerator1
          (bind _result_2 (Math|Float|NegateFloat DeltaSeconds :!label _label)
            (:%20%20
              (CallFunction|ChangeHealth _result_2))))
        (:NewEnumerator2
          (goto _label))
        (:NewEnumerator3
          (CallFunction|DiseaseEffect DeltaSeconds)
          (goto _label))))))

(fn ConstructionScript
  (Components|SkeletalMesh|SetSkeletalMeshAsset (Variables|Default|GetPatient) (Variables|Character|GetPatientModel)))

(fn ReceiveJoke
  (params (HealBy :type Float%20%28double-precision%29) (UsedJoke :type E_Jokes%20Enum :default "NewEnumerator8"))
  (if (Utilities|Enum|Equal(Enum) UsedJoke (Variables|Default|GetFavouriteJoke))
    (CallFunction|ChangeHealth (* HealBy 2.0))
    (else
      (CallFunction|ChangeHealth HealBy))))

(fn ChangeHealth
  (params (Change :type Float%20%28double-precision%29))
  (if (<= (+ (Variables|Default|GetCurrentHealth) Change) 0.0)
    (Variables|Default|SetCurrentHealth 0.0)
    (Variables|Default|SetStatus "NewEnumerator2")
    (elif (>= (+ (Variables|Default|GetCurrentHealth) Change) 1e+02)
      (Variables|Default|SetCurrentHealth 1e+02)
      (Variables|Default|SetStatus "NewEnumerator1")
      (else
        (Variables|Default|SetCurrentHealth (+ (Variables|Default|GetCurrentHealth) Change))))))

(fn DiseaseEffect
  (params (DeltaTime :type Float%20%28double-precision%29))
  (switch Utilities|FlowControl|Switch|SwitchonE_Diseases (Variables|Default|GetHasDisease)
    (:NewEnumerator3
      (if (and (Variables|Default|GetClownIsClose) (not (Variables|/Game/ThirdPerson/Blueprints/BP_ThirdPersonCharacter.BP_ThirdPersonCharacter_C|GetIsInfected (Variables|Default|GetClown))))
        (bind _output_get (Variables|Default|SetDiseaseTimer (+ DeltaTime (Variables|Default|GetDiseaseTimer))))
        (if (>= _output_get (Math|Conversions|ToFloat(Integer) (Variables|Default|GetDiseaseTime)))
          (Variables|/Game/ThirdPerson/Blueprints/BP_ThirdPersonCharacter.BP_ThirdPersonCharacter_C|SetIsInfected (Variables|Default|GetClown) true)
          (Development|PrintString "I GOT SICK"))))))