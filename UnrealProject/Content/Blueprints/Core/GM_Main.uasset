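; Main game mode that shows the main menu and removes the player character on the MainMenu level, and runs a timed round on other levels.
; Gameplay levels create the HUD, start the timer and pass the game mode to the suitcase to set available jokes.
; A one-second Delay loop updates the timer text and calls Countdown until time expires.
; Game over then shows its widget and cursor, disables character movement and hides timer and joke widgets.
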(event Custom|BeginGameTimer
  (bind _returnvalue (Game|GetPlayerController 0))
  (bind _w_mainhud_ref (Variables|Default|GetW_MainHUD_REF))
  ;[1 1 1] Begin game timer
  (Variables|/Game/HUD/W_GameTimer.W_GameTimer_C|SetTimerText (Variables|/Game/HUD/W_MainHUD.W_MainHUD_C|GetW_GameTimer (Variables|Default|GetW_MainHUD_REF)) (Utilities|TimeInfotoText) :!label _label)
  (bind _isgameover (CallFunction|Countdown))
  (bind _output_get (Variables|Default|SetIs%20Game%20Over _isgameover))
  (if (not _output_get)
    (Utilities|FlowControl|Delay 1.0)
    (goto _label)
    (else
      (bind _returnvalue_2 (UserInterface|CreateWidget "/Game/HUD/W_GameOver.W_GameOver_C" _returnvalue))
      (bind _output_get_2 (Variables|Default|SetW_GameOverREF _returnvalue_2))
      (UserInterface|Viewport|AddtoViewport _output_get_2 0)
      (Variables|/Script/Engine.PlayerController|SetbShowMouseCursor _returnvalue true)
      (bind _asbp_third_person_character (Utilities|Casting|CastToBP_ThirdPersonCharacter (Game|GetPlayerCharacter 0)))
      (Pawn|Components|CharacterMovement|SetMovementMode (Variables|/Script/Engine.Character|GetCharacterMovement _asbp_third_person_character) "MOVE_None" 0)
      (Widget|SetVisibility (Variables|/Game/HUD/W_MainHUD.W_MainHUD_C|GetW_GameTimer _w_mainhud_ref) "Hidden")
      (Widget|SetVisibility (Variables|/Game/HUD/W_MainHUD.W_MainHUD_C|GetW_SelectedJokes _w_mainhud_ref) "Hidden"))))

(event EventBeginPlay
  (bind _returnvalue (Game|GetPlayerController 0))
  (bind _returnvalue_2 (Game|GetCurrentLevelName true))
  (if (Utilities|Enum|Equal(Enum) _returnvalue_2 "MainMenu")
    (bind _returnvalue_3 (UserInterface|CreateWidget "/Game/HUD/W_MainMenu.W_MainMenu_C" _returnvalue))
    (UserInterface|Viewport|AddtoViewport _returnvalue_3 0)
    (bind _asbp_third_person_character (Utilities|Casting|CastToBP_ThirdPersonCharacter (Game|Player|GetPlayerPawn 0)))
    (Actor|DestroyActor _asbp_third_person_character)
    (else
      (bind _returnvalue_4 (UserInterface|CreateWidget "/Game/HUD/W_MainHUD.W_MainHUD_C" _returnvalue))
      (bind _output_get (Variables|Default|SetW_MainHUD_REF _returnvalue_4))
      (UserInterface|Viewport|AddtoViewport _output_get 0)
      (CallFunction|BeginGameTimer)
      (bind _returnvalue_5 (Actor|GetActorOfClass "/Game/Blueprints/BP_Suitcase.BP_Suitcase_C"))
      (if (Utilities|IsValid _returnvalue_5)
        (Default|SetAvailableJokes _returnvalue_5 self)))))

(fn ConstructionScript)

(fn Countdown
  (if (== (Variables|Default|GetTimerSeconds) 0)
    (if (> (Variables|Default|GetTimerMinutes) 0)
      (Variables|Default|SetTimerMinutes (- (Variables|Default|GetTimerMinutes) 1))
      (Variables|Default|SetTimerSeconds 59)
      (else
        (return true)))
    (else
      (Variables|Default|SetTimerSeconds (- (Variables|Default|GetTimerSeconds) 1))))
  (return false))