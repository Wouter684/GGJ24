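; BP_DesinfectionRoom is a two-door decontamination chamber that cleans the player character as it passes through.
; Overlap boxes outside each door drive timelines that slide the paired panels open and closed, tracking door state and the last door used.
; When a door finishes closing with the character inside, it activates particles, waits briefly, opens the opposite door, then clears the character's active effects and calls CleanClown.
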(event OnComponentBeginOverlap(DoorOutside1Box)
  (params (OverlappedComponent :type Primitive%20Component%20Object%20Reference) (OtherActor :type Actor%20Object%20Reference) (OtherComp :type Primitive%20Component%20Object%20Reference) (OtherBodyIndex :type Integer) (bFromSweep :type Boolean) (SweepResult :type Hit%20Result%20Structure%20%28by%20ref%29))
  (bind _door1l (Variables|Default|GetDoor1L))
  (bind _door1r (Variables|Default|GetDoor1R))
  (bind _returnvalue (Transformation|GetRelativeTransform _door1r))
  (bind _returnvalue_2 (Transformation|GetRelativeTransform _door1l))
  ;[1 1 1] Open / Close Door 1
  (Utilities|Casting|CastToBP_ThirdPersonCharacter OtherActor)
  (Variables|Default|SetStateDoor1 "NewEnumerator1")
  (bind (_direction _rightdoory _leftdoory) (Timeline|Door1 Play)
    (:Update
      (Transformation|SetRelativeLocation _door1r (Math|Vector|MakeVector (.x (.location _returnvalue)) _rightdoory (.z (.location _returnvalue))) false false)
      (Transformation|SetRelativeLocation _door1l (Math|Vector|MakeVector (.x (.location _returnvalue_2)) _leftdoory (.z (.location _returnvalue_2))) false false)
      (Variables|Default|SetLast%20Opened%20Door 1))
    (:Finished
      (switch Utilities|FlowControl|Switch|SwitchonE_DoorState (Variables|Default|GetStateDoor1)
        (:NewEnumerator1
          (Variables|Default|SetStateDoor1 "NewEnumerator2"))
        (:NewEnumerator3
          (Variables|Default|SetStateDoor1 "NewEnumerator0")
          (CallFunction|DesinfectionSequence))))))

(event OnComponentEndOverlap(DesinfectionBox)
  (params (OverlappedComponent :type Primitive%20Component%20Object%20Reference) (OtherActor :type Actor%20Object%20Reference) (OtherComp :type Primitive%20Component%20Object%20Reference) (OtherBodyIndex :type Integer))
  ;[1 1 1] Enter desinfection chamber
  (Utilities|Casting|CastToBP_ThirdPersonCharacter OtherActor)
  (Variables|Default|SetInsideDesinfection false))

(event OnComponentEndOverlap(DoorOutside1Box)
  (params (OverlappedComponent :type Primitive%20Component%20Object%20Reference) (OtherActor :type Actor%20Object%20Reference) (OtherComp :type Primitive%20Component%20Object%20Reference) (OtherBodyIndex :type Integer))
  (bind _door1l (Variables|Default|GetDoor1L))
  (bind _door1r (Variables|Default|GetDoor1R))
  (bind _returnvalue (Transformation|GetRelativeTransform _door1r))
  (bind _returnvalue_2 (Transformation|GetRelativeTransform _door1l))
  ;[1 1 1] Open / Close Door 1
  (Utilities|Casting|CastToBP_ThirdPersonCharacter OtherActor)
  (Variables|Default|SetStateDoor1 "NewEnumerator3")
  (bind (_direction _rightdoory _leftdoory) (Timeline|Door1 Reverse)
    (:Update
      (Transformation|SetRelativeLocation _door1r (Math|Vector|MakeVector (.x (.location _returnvalue)) _rightdoory (.z (.location _returnvalue))) false false)
      (Transformation|SetRelativeLocation _door1l (Math|Vector|MakeVector (.x (.location _returnvalue_2)) _leftdoory (.z (.location _returnvalue_2))) false false)
      (Variables|Default|SetLast%20Opened%20Door 1))
    (:Finished
      (switch Utilities|FlowControl|Switch|SwitchonE_DoorState (Variables|Default|GetStateDoor1)
        (:NewEnumerator1
          (Variables|Default|SetStateDoor1 "NewEnumerator2"))
        (:NewEnumerator3
          (Variables|Default|SetStateDoor1 "NewEnumerator0")
          (CallFunction|DesinfectionSequence))))))

(event OnComponentBeginOverlap(DoorOutside2Box)
  (params (OverlappedComponent :type Primitive%20Component%20Object%20Reference) (OtherActor :type Actor%20Object%20Reference) (OtherComp :type Primitive%20Component%20Object%20Reference) (OtherBodyIndex :type Integer) (bFromSweep :type Boolean) (SweepResult :type Hit%20Result%20Structure%20%28by%20ref%29))
  (bind _door2r (Variables|Default|GetDoor2R))
  (bind _door2l (Variables|Default|GetDoor2L))
  (bind _returnvalue (Transformation|GetRelativeTransform _door2l))
  (bind _returnvalue_2 (Transformation|GetRelativeTransform _door2r))
  ;[1 1 1] Open / Close Door 2
  (Utilities|Casting|CastToBP_ThirdPersonCharacter OtherActor)
  (Variables|Default|SetStateDoor2 "NewEnumerator1")
  (bind (_direction _rightdoory _leftdoory) (Timeline|Door%202 Play)
    (:Update
      (Transformation|SetRelativeLocation _door2r (Math|Vector|MakeVector (.x (.location _returnvalue_2)) _rightdoory (.z (.location _returnvalue_2))) false false)
      (Transformation|SetRelativeLocation _door2l (Math|Vector|MakeVector (.x (.location _returnvalue)) _leftdoory (.z (.location _returnvalue))) false false)
      (Variables|Default|SetLast%20Opened%20Door 2))
    (:Finished
      (switch Utilities|FlowControl|Switch|SwitchonE_DoorState (Variables|Default|GetStateDoor2)
        (:NewEnumerator1
          (Variables|Default|SetStateDoor2 "NewEnumerator2"))
        (:NewEnumerator3
          (Variables|Default|SetStateDoor2 "NewEnumerator0")
          (CallFunction|DesinfectionSequence))))))

(event OnComponentEndOverlap(DoorOutside2Box)
  (params (OverlappedComponent :type Primitive%20Component%20Object%20Reference) (OtherActor :type Actor%20Object%20Reference) (OtherComp :type Primitive%20Component%20Object%20Reference) (OtherBodyIndex :type Integer))
  (bind _door2r (Variables|Default|GetDoor2R))
  (bind _door2l (Variables|Default|GetDoor2L))
  (bind _returnvalue (Transformation|GetRelativeTransform _door2l))
  (bind _returnvalue_2 (Transformation|GetRelativeTransform _door2r))
  ;[1 1 1] Open / Close Door 2
  (Utilities|Casting|CastToBP_ThirdPersonCharacter OtherActor)
  (Variables|Default|SetStateDoor2 "NewEnumerator3")
  (bind (_direction _rightdoory _leftdoory) (Timeline|Door%202 Reverse)
    (:Update
      (Transformation|SetRelativeLocation _door2r (Math|Vector|MakeVector (.x (.location _returnvalue_2)) _rightdoory (.z (.location _returnvalue_2))) false false)
      (Transformation|SetRelativeLocation _door2l (Math|Vector|MakeVector (.x (.location _returnvalue)) _leftdoory (.z (.location _returnvalue))) false false)
      (Variables|Default|SetLast%20Opened%20Door 2))
    (:Finished
      (switch Utilities|FlowControl|Switch|SwitchonE_DoorState (Variables|Default|GetStateDoor2)
        (:NewEnumerator1
          (Variables|Default|SetStateDoor2 "NewEnumerator2"))
        (:NewEnumerator3
          (Variables|Default|SetStateDoor2 "NewEnumerator0")
          (CallFunction|DesinfectionSequence))))))

(event OnComponentBeginOverlap(DesinfectionBox)
  (params (OverlappedComponent :type Primitive%20Component%20Object%20Reference) (OtherActor :type Actor%20Object%20Reference) (OtherComp :type Primitive%20Component%20Object%20Reference) (OtherBodyIndex :type Integer) (bFromSweep :type Boolean) (SweepResult :type Hit%20Result%20Structure%20%28by%20ref%29))
  ;[1 1 1] Enter desinfection chamber
  (bind _asbp_third_person_character (Utilities|Casting|CastToBP_ThirdPersonCharacter OtherActor))
  (Variables|Default|SetClown _asbp_third_person_character)
  (Variables|Default|SetInsideDesinfection true))

(event Custom|Door_2
  (bind _door2r (Variables|Default|GetDoor2R))
  (bind _door2l (Variables|Default|GetDoor2L))
  (bind _returnvalue (Transformation|GetRelativeTransform _door2l))
  (bind _returnvalue_2 (Transformation|GetRelativeTransform _door2r))
  ;[1 1 1] Open / Close Door 2
  (bind (_direction _rightdoory _leftdoory) (Timeline|Door%202 Play)
    (:Update
      (Transformation|SetRelativeLocation _door2r (Math|Vector|MakeVector (.x (.location _returnvalue_2)) _rightdoory (.z (.location _returnvalue_2))) false false)
      (Transformation|SetRelativeLocation _door2l (Math|Vector|MakeVector (.x (.location _returnvalue)) _leftdoory (.z (.location _returnvalue))) false false)
      (Variables|Default|SetLast%20Opened%20Door 2))
    (:Finished
      (switch Utilities|FlowControl|Switch|SwitchonE_DoorState (Variables|Default|GetStateDoor2)
        (:NewEnumerator1
          (Variables|Default|SetStateDoor2 "NewEnumerator2"))
        (:NewEnumerator3
          (Variables|Default|SetStateDoor2 "NewEnumerator0")
          (CallFunction|DesinfectionSequence))))))

(event Custom|Door_1
  (bind _door1l (Variables|Default|GetDoor1L))
  (bind _door1r (Variables|Default|GetDoor1R))
  (bind _returnvalue (Transformation|GetRelativeTransform _door1r))
  (bind _returnvalue_2 (Transformation|GetRelativeTransform _door1l))
  ;[1 1 1] Open / Close Door 1
  (bind (_direction _rightdoory _leftdoory) (Timeline|Door1 Play)
    (:Update
      (Transformation|SetRelativeLocation _door1r (Math|Vector|MakeVector (.x (.location _returnvalue)) _rightdoory (.z (.location _returnvalue))) false false)
      (Transformation|SetRelativeLocation _door1l (Math|Vector|MakeVector (.x (.location _returnvalue_2)) _leftdoory (.z (.location _returnvalue_2))) false false)
      (Variables|Default|SetLast%20Opened%20Door 1))
    (:Finished
      (switch Utilities|FlowControl|Switch|SwitchonE_DoorState (Variables|Default|GetStateDoor1)
        (:NewEnumerator1
          (Variables|Default|SetStateDoor1 "NewEnumerator2"))
        (:NewEnumerator3
          (Variables|Default|SetStateDoor1 "NewEnumerator0")
          (CallFunction|DesinfectionSequence))))))

(event Custom|Desinfection%20Sequence
  (bind _clown (Variables|Default|GetClown))
  ;[1 1 1] Desinfection Sequence
  (if (Variables|Default|GetInsideDesinfection)
    (Components|Activation|Activate (Variables|Default|GetDesinfectParticles) false)
    (Utilities|FlowControl|Delay 2.0)
    (if (== (Variables|Default|GetLast%20Opened%20Door) 1)
      (CallFunction|Door2)
      (else
        (CallFunction|Door1)))
    (Utilities|Array|Clear (Variables|/Game/ThirdPerson/Blueprints/BP_ThirdPersonCharacter.BP_ThirdPersonCharacter_C|GetActiveEffects _clown))
    (Default|CleanClown _clown)))

(fn ConstructionScript)