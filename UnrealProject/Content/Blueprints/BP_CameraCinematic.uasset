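; BP_CameraCinematic is a camera actor that rides with a referenced elevator, presumably for cinematic shots.
; Its construction script attaches it to the elevator, then places the camera component at the elevator root's X and Y plus the LocationCamera offset, using that variable's Z as an absolute world height.
; RotationCamera sets the component's relative rotation, and the event graph has no runtime logic.
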(event EventBeginPlay)

(fn ConstructionScript
  (bind _elevatorref (Variables|Default|GetElevatorREF))
  (bind _cameracomponent (Variables|CameraActor|GetCameraComponent))
  (bind _locationcamera (Variables|Default|GetLocationCamera))
  (bind (_x _y _z) (Math|Vector|BreakVector _locationcamera))
  (bind _defaultsceneroot (Variables|/Game/Blueprints/BP_Elevator.BP_Elevator_C|GetDefaultSceneRoot _elevatorref))
  (bind _returnvalue (Transformation|GetWorldLocation _defaultsceneroot))
  (Transformation|AttachActorToActor _elevatorref "None" "KeepRelative" "KeepRelative" "KeepRelative" true)
  (Transformation|SetWorldLocation _cameracomponent (Math|Vector|MakeVector (+ (.x _returnvalue) _x) (+ (.y _returnvalue) _y) _z) false false)
  (Transformation|SetRelativeRotation _cameracomponent (Variables|Default|GetRotationCamera) false false))