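; Elevator actor that serves as a level exit, with a button to open its doors and a trigger that loads the next level.
; Overlapping the button collision enables input and shows a prompt, letting the player press Use to open closed doors.
; Timelines slide both doors by lerping from their current relative locations and track the open state.
; Entering the next-level collision closes the doors, then opens the named level after a short delay.
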(event OnComponentBeginOverlap(ButtonCollision)
  (params (OverlappedComponent :type Primitive%20Component%20Object%20Reference) (OtherActor :type Actor%20Object%20Reference) (OtherComp :type Primitive%20Component%20Object%20Reference) (OtherBodyIndex :type Integer) (bFromSweep :type Boolean) (SweepResult :type Hit%20Result%20Structure%20%28by%20ref%29))
  ;[1 1 1] Elevator button logic
  (bind _asbp_third_person_character (Utilities|Casting|CastToBP_ThirdPersonCharacter (Game|GetPlayerCharacter 0)))
  (if (== _asbp_third_person_character OtherActor)
    (Input|EnableInput (Game|GetPlayerController 0))
    (Rendering|SetVisibility (Variables|Default|GetButtonInteraction) true false)))

(event OnComponentBeginOverlap(NextLevelCollision)
  (params (OverlappedComponent :type Primitive%20Component%20Object%20Reference) (OtherActor :type Actor%20Object%20Reference) (OtherComp :type Primitive%20Component%20Object%20Reference) (OtherBodyIndex :type Integer) (bFromSweep :type Boolean) (SweepResult :type Hit%20Result%20Structure%20%28by%20ref%29))
  ;[1 1 1] Next level transition logic
  (bind _asbp_third_person_character (Utilities|Casting|CastToBP_ThirdPersonCharacter (Game|GetPlayerCharacter 0)))
  (if (== _asbp_third_person_character OtherActor)
    (CallFunction|DoorsClose)
    (Utilities|FlowControl|Delay 3.0)
    (Game|OpenLevel(byName) (Variables|Default|GetNextLevelName))))

(event OnComponentEndOverlap(ButtonCollision)
  (params (OverlappedComponent :type Primitive%20Component%20Object%20Reference) (OtherActor :type Actor%20Object%20Reference) (OtherComp :type Primitive%20Component%20Object%20Reference) (OtherBodyIndex :type Integer))
  ;[1 1 1] Elevator button logic
  (bind _asbp_third_person_character (Utilities|Casting|CastToBP_ThirdPersonCharacter (Game|GetPlayerCharacter 0)))
  (if (== _asbp_third_person_character OtherActor)
    (Input|DisableInput (Game|GetPlayerController 0))
    (Rendering|SetVisibility (Variables|Default|GetButtonInteraction) false false)))

(event Custom|DoorsClose
  ;[1 1 1] Elevator doors open/close
  (bind _rate (Timeline|Timeline_0 ReverseFromEnd)
    (:Update
      (Transformation|SetRelativeLocation (Variables|Default|GetDoorRight) (Math|Vector|Lerp(Vector) (Variables|/Script/Engine.SceneComponent|GetRelativeLocation (Variables|Default|GetDoorRight)) "250.000000,0.000000,0.000000" _rate) false false)
      (Transformation|SetRelativeLocation (Variables|Default|GetDoorLeft) (Math|Vector|Lerp(Vector) (Variables|/Script/Engine.SceneComponent|GetRelativeLocation (Variables|Default|GetDoorLeft)) "75.000000,0.000000,0.000000" _rate) false false))
    (:Finished
      (Variables|Default|SetIsDoorOpen false))))

(event Custom|DoorsOpen
  ;[1 1 1] Elevator doors open/close
  (bind _rate (Timeline|Timeline PlayFromStart)
    (:Update
      (Transformation|SetRelativeLocation (Variables|Default|GetDoorLeft) (Math|Vector|Lerp(Vector) (Variables|/Script/Engine.SceneComponent|GetRelativeLocation (Variables|Default|GetDoorLeft)) "0, 0, 0" _rate) false false)
      (Transformation|SetRelativeLocation (Variables|Default|GetDoorRight) (Math|Vector|Lerp(Vector) (Variables|/Script/Engine.SceneComponent|GetRelativeLocation (Variables|Default|GetDoorRight)) "315.000000,0.000000,0.000000" _rate) false false))
    (:Finished
      (Variables|Default|SetIsDoorOpen true))))

(event Input|EnhancedActionEvents|EnhancedInputActionIA_Use
  (params (ActionValue :type Boolean) (ElapsedSeconds :type Float%20%28double-precision%29) (TriggeredSeconds :type Float%20%28double-precision%29) (InputAction :type Input%20Action%20Object%20Reference :default "/Game/ThirdPerson/Input/Actions/IA_Use.IA_Use"))
  (:Started
    (if (not (Variables|Default|GetIsDoorOpen))
      (CallFunction|DoorsOpen))))

(fn ConstructionScript)