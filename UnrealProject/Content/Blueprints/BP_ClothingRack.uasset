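; Interactable clothing rack that displays an outfit and lets the player character swap clothes with it.
; The construction script finds the outfit named by ContainsOutfit in AllOutfits and shows its mesh on the Suit.
; Overlapping the collision box enables input and a button prompt, so IA_Use calls SwapClothes on the character with the rack and its outfit.
; GetNewOutfit stores the outfit passed to it and updates the displayed mesh.
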(event OnComponentBeginOverlap(Collision)
  (params (OverlappedComponent :type Primitive%20Component%20Object%20Reference) (OtherActor :type Actor%20Object%20Reference) (OtherComp :type Primitive%20Component%20Object%20Reference) (OtherBodyIndex :type Integer) (bFromSweep :type Boolean) (SweepResult :type Hit%20Result%20Structure%20%28by%20ref%29))
  ;[1 1 1] Collision box
  (bind _asbp_third_person_character (Utilities|Casting|CastToBP_ThirdPersonCharacter OtherActor))
  (Variables|Default|SetClown _asbp_third_person_character)
  (Input|EnableInput (Game|GetPlayerController 0))
  (Rendering|SetVisibility (Variables|Default|GetButtonPrompt) true false))

(event OnComponentEndOverlap(Collision)
  (params (OverlappedComponent :type Primitive%20Component%20Object%20Reference) (OtherActor :type Actor%20Object%20Reference) (OtherComp :type Primitive%20Component%20Object%20Reference) (OtherBodyIndex :type Integer))
  ;[1 1 1] Collision box
  (Utilities|Casting|CastToBP_ThirdPersonCharacter OtherActor)
  (Input|DisableInput (Game|GetPlayerController 0))
  (Rendering|SetVisibility (Variables|Default|GetButtonPrompt) false false))

(event Custom|Get%20New%20Outfit
  (params (New%20Outfit :type BPS%20Outfit%20Structure))
  ;[1 1 1] Swap Clothes
  (bind _output_get (Variables|Default|SetMy%20Outfit New%20Outfit))
  (Components|SkeletalMesh|SetSkeletalMeshAsset (Variables|Default|GetSuit) (Utilities|Struct|BreakBPS_Outfit _output_get)))

(event Input|EnhancedActionEvents|EnhancedInputActionIA_Use
  (params (ActionValue :type Boolean) (ElapsedSeconds :type Float%20%28double-precision%29) (TriggeredSeconds :type Float%20%28double-precision%29) (InputAction :type Input%20Action%20Object%20Reference :default "/Game/ThirdPerson/Input/Actions/IA_Use.IA_Use"))
  ;[1 1 1] Swap Clothes
  (:Started
    (Default|SwapClothes (Variables|Default|GetClown) self (Variables|Default|GetMy%20Outfit))))

(fn ConstructionScript
  (bind _array_element (Utilities|Array|ForEachLoopwithBreak (Variables|Default|GetAll%20Outfits))
    (:LoopBody
      (if (Utilities|Enum|Equal(Enum) (Utilities|Struct|BreakBPS_Outfit _array_element) (Variables|Default|GetContainsOutfit))
        (bind _output_get (Variables|Default|SetMy%20Outfit _array_element))
        (Components|SkeletalMesh|SetSkeletalMeshAsset (Variables|Default|GetSuit) (Utilities|Struct|BreakBPS_Outfit _output_get))))))