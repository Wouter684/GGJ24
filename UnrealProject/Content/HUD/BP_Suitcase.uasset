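; BP_Suitcase is an interactable suitcase that opens and closes the player's joke inventory widget.
; Entering its trigger box enables input and caches the character's JokeInventoryWidget; leaving also calls EnableInput, so input is never disabled here.
; The gamepad bottom face button toggles widget visibility and the character's SuitcaseOpen flag, resetting selection to the first cell on opening.
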(event OnComponentBeginOverlap(TriggerBox)
  (params (OverlappedComponent :type Primitive%20Component%20Object%20Reference) (OtherActor :type Actor%20Object%20Reference) (OtherComp :type Primitive%20Component%20Object%20Reference) (OtherBodyIndex :type Integer) (bFromSweep :type Boolean) (SweepResult :type Hit%20Result%20Structure%20%28by%20ref%29))
  (bind _asbp_third_person_character (Utilities|Casting|CastToBP_ThirdPersonCharacter OtherActor))
  (Input|EnableInput (Game|GetPlayerController 0))
  (if (not (Utilities|IsValid (Variables|Default|GetJoke%20Inventory%20Widget)))
    (Variables|Default|SetJoke%20Inventory%20Widget (Variables|/Game/ThirdPerson/Blueprints/BP_ThirdPersonCharacter.BP_ThirdPersonCharacter_C|GetjokeInventoryWidget _asbp_third_person_character))))

(event OnComponentEndOverlap(TriggerBox)
  (params (OverlappedComponent :type Primitive%20Component%20Object%20Reference) (OtherActor :type Actor%20Object%20Reference) (OtherComp :type Primitive%20Component%20Object%20Reference) (OtherBodyIndex :type Integer))
  (Utilities|Casting|CastToBP_ThirdPersonCharacter OtherActor)
  (Input|EnableInput (Game|GetPlayerController 0)))

(event Input|GamepadEvents|GamepadFaceButtonBottom
  (params (Key :type Key%20Structure :default "None"))
  (bind _returnvalue (Game|Player|GetPlayerPawn 0))
  (bind _joke_inventory_widget (Variables|Default|GetJoke%20Inventory%20Widget))
  (bind _joke_inventory_widget_2 (Variables|Default|GetJoke%20Inventory%20Widget))
  (:Pressed
    (if (== (Variables|/Script/UMG.Widget|GetVisibility _joke_inventory_widget) 0)
      (Variables|/Script/UMG.Widget|SetVisibility _joke_inventory_widget "Hidden")
      (bind _asbp_third_person_character (Utilities|Casting|CastToBP_ThirdPersonCharacter _returnvalue))
      (Variables|/Game/ThirdPerson/Blueprints/BP_ThirdPersonCharacter.BP_ThirdPersonCharacter_C|SetsuitcaseOpen _asbp_third_person_character false)
      (else
        (Variables|/Script/UMG.Widget|SetVisibility _joke_inventory_widget "Visible")
        (bind _asbp_third_person_character_2 (Utilities|Casting|CastToBP_ThirdPersonCharacter _returnvalue))
        (Variables|/Game/ThirdPerson/Blueprints/BP_ThirdPersonCharacter.BP_ThirdPersonCharacter_C|SetsuitcaseOpen _asbp_third_person_character_2 true)
        (Variables|/Game/HUD/W_JokeInventory.W_JokeInventory_C|SetRowIndex _joke_inventory_widget_2 0)
        (Variables|/Game/HUD/W_JokeInventory.W_JokeInventory_C|SetColumnIndex _joke_inventory_widget_2 0)
        (Default|ChangeSelection _joke_inventory_widget_2)))))

(fn ConstructionScript)